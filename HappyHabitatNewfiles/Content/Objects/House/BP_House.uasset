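; BP_House is a house actor that switches the player's view between its own camera and the static player camera.
; On BeginPlay it enables input for player 0 and adds the house selection Enhanced Input mapping context.
; SelectHouse toggles IsInHouseView, blending the view target to the owner of HouseCamera or of the BP_StaticCameraPlayer's StaticCamera.
; A short delay precedes each flag flip.
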(event Custom|SelectHouse
  ;[0.01667 0.1275 0.15 0.5] HouseSelection
  (bind _returnvalue (Actor|GetActorOfClass "/Game/Cameras/BP_StaticCameraPlayer.BP_StaticCameraPlayer_C"))
  (if (Variables|Default|GetbIsInHouseView)
    (Game|Player|SetViewTargetwithBlend (Game|GetPlayerController 0) (Components|GetOwner (Variables|/Game/Cameras/BP_StaticCameraPlayer.BP_StaticCameraPlayer_C|GetStaticCamera _returnvalue)) 1.0 "VTBlend_Linear" 0.0 false)
    (Utilities|FlowControl|Delay 0.2)
    (Variables|Default|SetbIsInHouseView false)
    (else
      (Game|Player|SetViewTargetwithBlend (Game|GetPlayerController 0) (Components|GetOwner (Variables|Default|GetHouseCamera)) 1.0 "VTBlend_Linear" 0.0 false)
      (Utilities|FlowControl|Delay 0.2)
      (Variables|Default|SetbIsInHouseView true))))

(event Collision|EventActorBeginOverlap
  (params (OtherActor :type Actor%20Object%20Reference)))

(event EventBeginPlay
  ;[0.15 0.05275 0.1236 0.5] ControllerMapping
  (Input|EnableInput (Game|GetPlayerController 0))
  (bind _asplayer_controller (Utilities|Casting|CastToPlayerController (Game|GetPlayerController 0)))
  (Utilities|IsValid (PlayerController|LocalPlayerSubsystems|GetEnhancedInputLocalPlayerSubsystem _asplayer_controller)
    (:Is%20Valid
      (Input|AddMappingContext (PlayerController|LocalPlayerSubsystems|GetEnhancedInputLocalPlayerSubsystem _asplayer_controller) "/Game/InputMapping/IMC_HouseSelection.IMC_HouseSelection" 0 "(bIgnoreAllPressedKeysUntilRelease=True,bForceImmediately=False,bNotifyUserSettings=False)"))))

(fn ConstructionScript)
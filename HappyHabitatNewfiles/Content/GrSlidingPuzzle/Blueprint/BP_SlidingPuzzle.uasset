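; Sliding-tile picture puzzle actor that shows a victory widget and plays a sound when solved.
; Construction script builds a scaled grid of box slots and tiles with one gap, offsets the texture per tile material, optionally shuffles tiles, and positions BP_PuzzleCamera.
; Clicking a tile sphere-overlaps nearby slots, picks an unoccupied one and slides the tile there on a timeline.
; After each move, overlap tests between tiles and their original slots check completion.
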(event Custom|MeshClick
  (params (TouchedComponent :type Primitive%20Component%20Object%20Reference) (ButtonPressed :type Key%20Structure :default "None"))
  (bind _output_get (Variables|Default|SetMeshOnClick TouchedComponent))
  (EventDispatchers|BindEventtoOnClicked _output_get (delegate Custom|MeshClick))
  (bind (_next _returnvalue) (CallFunction|FNextBlock))
  (if _returnvalue
    (CallFunction|FMoveto _next)
    (Utilities|IsValid (Variables|Default|GetMoveToPoint)
      (:Is%20Valid
        (CallFunction|Moveto)))))

(event Custom|BindClickMesh
  (for _array_element (Variables|Default|GetStaticMeshComp)
    (EventDispatchers|BindEventtoOnClicked _array_element (delegate Custom|MeshClick))))

(event Custom|RemoveAndClose
  (bind _returnvalue (Game|GetPlayerController 0))
  ;[1 0.04223 0] bind event to close the widget
  (Variables|/Script/Engine.PlayerController|SetbShowMouseCursor _returnvalue false)
  (Input|SetInputModeGameOnly _returnvalue false)
  (Widget|RemovefromParent (Variables|Default|GetWG_Victory)))

(event Custom|MoveTo
  (Variables|/Script/Engine.PlayerController|SetbEnableClickEvents (Game|GetPlayerController 0) false)
  (Variables|Default|SetMove%20toStart (Variables|/Script/Engine.SceneComponent|GetRelativeLocation (Variables|Default|GetMeshOnClick)))
  (bind _alpha (Timeline|Timeline_0 PlayFromStart)
    (:Update
      (Transformation|SetRelativeLocation (Variables|Default|GetMeshOnClick) (Math|Vector|Lerp(Vector) (Variables|Default|GetMove%20toStart) (Variables|/Script/Engine.SceneComponent|GetRelativeLocation (Variables|Default|GetMoveToPoint)) _alpha) false false))
    (:Finished
      (Variables|/Script/Engine.PlayerController|SetbEnableClickEvents (Game|GetPlayerController 0) true)
      ;[0.01356 0.47 0.0546] Checking the position of the blocks. Is the puzzle solved?
      (bind _solved (CallFunction|PuzzleSolved?))
      ;[0.8833 0.5249 1] With the correct solution of the puzzle, we create some actions. In this case, the "Victory" widget is created with the playback of a sound file.
      (if _solved
        (Audio|PlaySoundatLocation (Variables|Default|GetSoundVictory) (Transformation|GetActorLocation) "0, 0, 0" (Variables|Default|GetVolume) (Variables|Default|GetPitch) 0.0 0 0 0 0)
        (bind _returnvalue (UserInterface|CreateWidget "/Game/GrSlidingPuzzle/Widget/WG_Win.WG_Win_C" 0 self))
        (bind _output_get (Variables|Default|SetWG_Victory _returnvalue))
        (UserInterface|Viewport|AddtoViewport _output_get 0)
        ;[1 0.04223 0] bind event to close the widget
        (EventDispatchers|BindEventtoDispWGButtonClose (delegate Custom|RemoveAndClose))
        ;[0.1401 0.42 0.3036] bind event for restart
        (EventDispatchers|BindEventtoDispWGButtonRestart (delegate Custom|Restart))))))

(event Custom|Restart
  ;[0.1401 0.42 0.3036] bind event for restart
  (Variables|Default|SetIsRandom? false)
  (CallFunction|FRandomPuzzle)
  (Widget|RemovefromParent (Variables|Default|GetWG_Victory)))

(event EventBeginPlay
  (bind _returnvalue (Game|GetPlayerController 0))
  (Utilities|FlowControl|Sequence
    (:then_0
      (Variables|/Script/Engine.PlayerController|SetbEnableClickEvents _returnvalue true)
      (Variables|/Script/Engine.PlayerController|SetbShowMouseCursor _returnvalue true))
    (:then_1
      (CallFunction|BindClickMesh))))

(fn ConstructionScript
  (bind _sizemesh (Variables|Default|GetSizeMesh))
  (bind _sizegrid (Variables|Default|GetSizeGrid))
  (bind _returnvalue (* _sizegrid _sizemesh))
  (bind _returnvalue_2 (/ _sizemesh 2.0))
  (bind _returnvalue_3 (/ _returnvalue 2.0))
  (bind _returnvalue_4 (- _returnvalue_3 _returnvalue_2))
  ;[1 0.5117 0.7859] Creating blocks for the puzzle
  (CallFunction|FSlidingPuzzle)
  ;[1 0.5556 0.07462] Set the size of the blocks for the puzzle
  (CallFunction|FScalePuzzle)
  ;[0.1601 0.525 0.03816] Making the location randomized by a block for clues
  (CallFunction|FRandomPuzzle)
  ;[0.8334 1 0.4463] Add a camera and set the position, rotation
  (bind _outactors (Actor|GetAllActorsOfClass "/Game/Cameras/BP_PuzzleCamera.BP_PuzzleCamera_C"))
  (Transformation|SetRelativeLocation (Variables|/Game/Cameras/BP_PuzzleCamera.BP_PuzzleCamera_C|GetPuzzleCamera (Utilities|Array|Get(acopy) _outactors)) (Math|Vector|MakeVector _returnvalue_4 _returnvalue_4 (Variables|Default|GetTargetArmLength)) false false)
  (Transformation|SetRelativeRotation (Variables|/Game/Cameras/BP_PuzzleCamera.BP_PuzzleCamera_C|GetPuzzleCamera (Utilities|Array|Get(acopy) _outactors)) "-90.000000,-90.000000, 0" false false))

(fn FSlidingPuzzle
  (bind _sizemesh (Variables|Default|GetSizeMesh))
  (bind _sizegrid (Variables|Default|GetSizeGrid))
  (bind _sizegrid_2 (Variables|Default|GetSizeGrid))
  (bind _list (Variables|Default|GetList))
  (bind _sizemesh_2 (Variables|Default|GetSizeMesh))
  (bind _staticmeshcomp (Variables|Default|GetStaticMeshComp))
  (bind _sizegrid_3 (Variables|Default|GetSizeGrid))
  (bind _sizemesh_3 (Variables|Default|GetSizeMesh))
  (bind _returnvalue (Math|Conversions|ToFloat(Integer) _sizegrid_2))
  (bind _returnvalue_2 (/ _sizemesh 4.0))
  (bind _returnvalue_3 (Math|Integer|Clamp(Integer) _sizegrid_3 3 32))
  (bind _returnvalue_4 (- _returnvalue_3 1))
  (bind _returnvalue_5 (/ 1.0 _returnvalue))
  (bind _arrayelement (Utilities|Array|ReverseforEachLoop _list)
    (:LoopBody
      (Components|DestroyComponent _arrayelement))
    (:Completed
      (Utilities|Array|Clear _list)
      (bind _arrayelement_2 (Utilities|Array|ReverseforEachLoop _staticmeshcomp)
        (:LoopBody
          (Components|DestroyComponent _arrayelement_2))
        (:Completed
          (Utilities|Array|Clear _staticmeshcomp)
          (for _index (range 0 _returnvalue_4)
            (Variables|Default|SetYgrid _index)
            (for _index_2 (range 0 _returnvalue_4)
              (Variables|Default|SetXgrid _index_2)
              (bind _returnvalue_6 (AddComponent|AddBoxComponent false (Math|Transform|MakeTransform (Math|Vector|MakeVector (* (Variables|Default|GetXgrid) _sizemesh_2) (* (Variables|Default|GetYgrid) _sizemesh_2) 2.0) "0, 0, 0" "1.000000,1.000000,1.000000")))
              (Components|Box|SetBoxExtent _returnvalue_6 (Math|Vector|MakeVector _returnvalue_2 _returnvalue_2 2.0) true)
              (Utilities|Array|Add (Variables|Default|GetList) _returnvalue_6)
              (if (not (and (== (- _sizegrid 1) (Variables|Default|GetYgrid)) (== (- _sizegrid 1) (Variables|Default|GetXgrid))))
                (bind _returnvalue_7 (AddComponent|AddStaticMeshComponent false (Math|Transform|MakeTransform (Math|Vector|MakeVector (* (Variables|Default|GetXgrid) _sizemesh_3) (* (Variables|Default|GetYgrid) _sizemesh_3) 0.0) "0,90.000000, 0" "1.000000,1.000000,1.000000")))
                (Components|StaticMesh|SetStaticMesh _returnvalue_7 (Variables|Default|GetMesh))
                (Utilities|Array|Add (Variables|Default|GetStaticMeshComp) _returnvalue_7)
                (bind _returnvalue_8 (Rendering|Material|CreateDynamicMaterialInstance _returnvalue_7 0 "/Game/GrSlidingPuzzle/Material/Mat_pazzle.Mat_pazzle" "None" :!class /Script/Engine.PrimitiveComponent))
                (Rendering|Material|SetTextureParameterValue _returnvalue_8 "PuzzleTexture" (Variables|Default|GetTextureName))
                (Rendering|Material|SetVectorParameterValueonMaterials _returnvalue_7 "TextureOffset" (Math|Vector|MakeVector (* (Variables|Default|GetXgrid) _returnvalue_5) (* (Variables|Default|GetYgrid) _returnvalue_5) _returnvalue))))))))))

(fn FRandomPuzzle
  (bind _location (LocalVariables|GetLocation))
  (if (Variables|Default|GetIsRandom?)
    (for _array_element (Variables|Default|GetList)
      (Utilities|Array|Add (LocalVariables|GetLocation) (Variables|/Script/Engine.SceneComponent|GetRelativeLocation _array_element)))
    (Utilities|Array|Shuffle (LocalVariables|GetLocation))
    (for _array_element_2 (Variables|Default|GetStaticMeshComp)
      (Transformation|SetRelativeLocation _array_element_2 (Utilities|Array|Get(acopy) _location) false false)
      (Utilities|Array|RemoveIndex _location))
    (return)
    (else
      (return))))

(fn FScalePuzzle
  (bind _scale (Variables|Default|GetScale))
  (bind _sizegrid (Variables|Default|GetSizeGrid))
  (bind _sizemesh (Variables|Default|GetSizeMesh))
  (bind _returnvalue (* _sizegrid _sizemesh))
  (bind _returnvalue_2 (/ _returnvalue _scale))
  (bind _returnvalue_3 (/ "1.000000,1.000000,1.000000" _returnvalue_2))
  (Transformation|SetActorScale3D (Math|Vector|MakeVector (.x _returnvalue_3) (.y _returnvalue_3) (.z _returnvalue_3)))
  (return))

(fn FMoveto
  (params (Input :type Array%20of%20Primitive%20Component%20Object%20References))
  (Variables|Default|SetMoveToPoint 0)
  (for _array_element Input
    (if (not (Collision|IsOverlappingActor _array_element self :!class /Script/Engine.PrimitiveComponent))
      (Variables|Default|SetMoveToPoint _array_element)
      (Audio|PlaySoundatLocation (Variables|Default|GetSound) (Transformation|GetActorLocation) "0, 0, 0" (Variables|Default|GetVolume) (Variables|Default|GetPitch) 0.0 0 0 0 0)))
  (return))

(fn PuzzleSolved?
  (bind (_array_element _array_index) (Utilities|Array|ForEachLoopwithBreak (Variables|Default|GetStaticMeshComp) :!label _label)
    (:LoopBody
      (if (not (Class|PrimitiveComponent|IsOverlappingComponent _array_element (Utilities|Array|Get(acopy) (Variables|Default|GetList) _array_index)))
        (LocalVariables|SetVariableSolved false)
        (goto _label Break)))
    (:Completed
      (return (LocalVariables|GetVariableSolved)))))

(fn FNextBlock
  (bind (_outcomponents _returnvalue) (Collision|SphereOverlapComponents (Transformation|GetWorldLocation (Variables|Default|GetMeshOnClick)) (* (* (* (/ (Variables|Default|GetSizeMesh) 2.0) (/ (/ (Variables|Default|GetSizeMesh) (Math|Conversions|ToFloat(Integer) (Variables|Default|GetSizeGrid))) (/ (Variables|Default|GetSizeMesh) 2.0))) (/ 1.0 (/ (* (Variables|Default|GetSizeGrid) (Variables|Default|GetSizeMesh)) (Variables|Default|GetScale)))) (Math|Conversions|ToFloat(Integer) (Variables|Default|GetSizeGrid))) (Utilities|Array|MakeArray "ObjectTypeQuery2") "/Script/Engine.BoxComponent"))
  (return _outcomponents _returnvalue))
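; BP_HouseSelector lets the player cycle through an array of houses with a triangle indicator and confirm one to trigger NPC dialogue.
; BeginPlay creates a hidden WBP_NPCDialogue widget shared with the DialogueManager, adds the house-selection Enhanced Input context and spawns the indicator above the first house.
; Delayed left/right inputs update the modulo-wrapped index and move the indicator.
; Confirming calls SelectHouse on the current BP_House and requests random dialogue, setting the widget Hidden in both branches.
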(event Input|EnhancedActionEvents|EnhancedInputActionIA_CycleRight
  (params (ActionValue :type Boolean) (ElapsedSeconds :type Float%20%28double-precision%29) (TriggeredSeconds :type Float%20%28double-precision%29) (InputAction :type Input%20Action%20Object%20Reference :default "/Game/InputMapping/IA_CycleRight.IA_CycleRight"))
  ;[0.6823 0.6451 0.1528 0.5] Cycling
  (Utilities|FlowControl|Delay 0.3)
  (Variables|Default|SetCurrentIndex (Math|Integer|%(Integer) (+ (Variables|Default|GetCurrentIndex) 1) (Utilities|Array|Length (Variables|Default|GetHouseArray))))
  (Variables|Default|SetSelectedHouse (Utilities|Array|Get(acopy) (Variables|Default|GetHouseArray) (Variables|Default|GetCurrentIndex)))
  (Transformation|SetActorLocation (Variables|Default|GetIndicator) (Math|Vector|MakeVector (.X (Math|Vector|BreakVector (Transformation|GetActorLocation (Utilities|Array|Get(acopy) (Variables|Default|GetHouseArray) (Variables|Default|GetCurrentIndex))))) (.Y (Math|Vector|BreakVector (Transformation|GetActorLocation (Utilities|Array|Get(acopy) (Variables|Default|GetHouseArray) (Variables|Default|GetCurrentIndex))))) 2.8e+02) false false))

(event Input|EnhancedActionEvents|EnhancedInputActionIA_CycleLeft
  (params (ActionValue :type Boolean) (ElapsedSeconds :type Float%20%28double-precision%29) (TriggeredSeconds :type Float%20%28double-precision%29) (InputAction :type Input%20Action%20Object%20Reference :default "/Game/InputMapping/IA_CycleLeft.IA_CycleLeft"))
  ;[0.6823 0.6451 0.1528 0.5] Cycling
  (Utilities|FlowControl|Delay 0.3)
  (bind _result (Math|Integer|DecrementInt (Variables|Default|GetCurrentIndex))
    (:%20%20
      (Variables|Default|SetCurrentIndex (Math|Integer|%(Integer) _result (Utilities|Array|Length (Variables|Default|GetHouseArray))))
      (Variables|Default|SetSelectedHouse (Utilities|Array|Get(acopy) (Variables|Default|GetHouseArray) (Variables|Default|GetCurrentIndex)))
      (Transformation|SetActorLocation (Variables|Default|GetIndicator) (Math|Vector|MakeVector (.X (Math|Vector|BreakVector (Transformation|GetActorLocation (Utilities|Array|Get(acopy) (Variables|Default|GetHouseArray) (Variables|Default|GetCurrentIndex))))) (.Y (Math|Vector|BreakVector (Transformation|GetActorLocation (Utilities|Array|Get(acopy) (Variables|Default|GetHouseArray) (Variables|Default|GetCurrentIndex))))) 2.8e+02) false false))))

(event Input|EnhancedActionEvents|EnhancedInputActionIA_SelectHouse
  (params (ActionValue :type Boolean) (ElapsedSeconds :type Float%20%28double-precision%29) (TriggeredSeconds :type Float%20%28double-precision%29) (InputAction :type Input%20Action%20Object%20Reference :default "/Game/InputMapping/IA_SelectHouse.IA_SelectHouse"))
  ;[0.04569 0.1213 0.15 0.5] HouseConfirm/DialogueBoxOpenClose
  (:Completed
    (if (Variables|Default|GetwidgetNOTvisible)
      (bind _asbp_house (Utilities|Casting|CastToBP_House (Variables|Default|GetSelectedHouse)))
      (Utilities|IsValid (Variables|Default|GetSelectedHouse)
        (:Is%20Valid
          (Default|SelectHouse _asbp_house)
          (bind _outactors (Actor|GetAllActorsOfClass "/Game/ABP_DialogueManager.ABP_DialogueManager_C"))
          (Variables|Default|SetWidgetON true)
          (Default|GetRandomDialogue (Utilities|Array|Get(acopy) _outactors))
          (Widget|SetVisibility (Variables|Default|GetDialogueWidgetReference) "Hidden"))
        (:Is%20Not%20Valid
          (Development|PrintString "HouseSelectionNotValid")))
      (else
        (bind _asbp_house_2 (Utilities|Casting|CastToBP_House (Variables|Default|GetSelectedHouse)))
        (Utilities|IsValid (Variables|Default|GetSelectedHouse)
          (:Is%20Valid
            (Default|SelectHouse _asbp_house_2)
            (bind _outactors_2 (Actor|GetAllActorsOfClass "/Game/ABP_DialogueManager.ABP_DialogueManager_C"))
            (Variables|Default|SetWidgetON false)
            (Default|GetRandomDialogue (Utilities|Array|Get(acopy) _outactors_2))
            (Widget|SetVisibility (Variables|Default|GetDialogueWidgetReference) "Hidden"))
          (:Is%20Not%20Valid
            (Development|PrintString "HouseSelectionNotValid")))))))

(event Collision|EventActorBeginOverlap
  (params (OtherActor :type Actor%20Object%20Reference))
  ;[0.6823 0.6451 0.1528 0.5] Cycling
)

(event EventBeginPlay
  (bind _housearray (Variables|Default|GetHouseArray))
  (bind _output (Utilities|Array|Get(acopy) _housearray))
  (bind _returnvalue (Transformation|GetActorLocation _output))
  (bind (_x _y _z) (Math|Vector|BreakVector _returnvalue))
  (bind _returnvalue_2 (+ _z 3.3e+02))
  (bind _returnvalue_3 (Math|Vector|MakeVector _x _y _returnvalue_2))
  ;[0.15 0.02094 0.1088 0.5] SpawnIndictator/PopulateArray
  (bind _returnvalue_4 (UserInterface|CreateWidget "/Game/WBP_NPCDialogue.WBP_NPCDialogue_C"))
  (bind _output_get (Variables|Default|SetDialogueWidgetReference _returnvalue_4))
  (bind _outactors (Actor|GetAllActorsOfClass "/Game/ABP_DialogueManager.ABP_DialogueManager_C"))
  (bind _output_get_2 (Variables|/Game/ABP_DialogueManager.ABP_DialogueManager_C|SetDialogueWidgetReferenc (Utilities|Array|Get(acopy) _outactors) _output_get))
  (UserInterface|Viewport|AddtoViewport _output_get_2 0)
  (Variables|/Script/UMG.Widget|SetVisibility (Variables|Default|GetDialogueWidgetReference) "Hidden")
  (Variables|Default|SetwidgetNOTvisible true)
  (Variables|Default|SetCurrentIndex 0)
  (Input|EnableInput (Game|GetPlayerController 0))
  (bind _asplayer_controller (Utilities|Casting|CastToPlayerController (Game|GetPlayerController 0)))
  (Utilities|IsValid (PlayerController|LocalPlayerSubsystems|GetEnhancedInputLocalPlayerSubsystem _asplayer_controller)
    (:Is%20Valid
      (Input|AddMappingContext (PlayerController|LocalPlayerSubsystems|GetEnhancedInputLocalPlayerSubsystem _asplayer_controller) "/Game/InputMapping/IMC_HouseSelection.IMC_HouseSelection" 0 "(bIgnoreAllPressedKeysUntilRelease=True,bForceImmediately=False,bNotifyUserSettings=False)")
      (bind _returnvalue_5 (Game|SpawnActorfromClass "/Game/BP_TriangleIndicator.BP_TriangleIndicator_C" (Math|Conversions|ToTransform(Vector) _returnvalue_3) "Undefined" "MultiplyWithRoot" 0 0))
      (bind _output_get_3 (Variables|Default|SetIndicator _returnvalue_5))
      (if true
        (Transformation|SetActorScale3D _output_get_3 "4.500000,4.500000,4.500000")
        (Transformation|SetActorLocation _returnvalue_3 false false)
        (else
          (Development|PrintString "IndicatorNOTset"))))))

(fn ConstructionScript)

(fn NewFunction)